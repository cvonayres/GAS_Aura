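; Potion bottle pickup that applies a gameplay effect to an actor overlapping its sphere.
; The construction script builds it from a data asset, setting mesh and liquid material by potion Type and copying in instant, duration, infinite and periodic effect classes.
; Type then sets the policies so only the matching effect applies on overlap, with infinite effects removed on end overlap.
; Sphere begin overlap hands the other actor to OnOverlap.
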(event OnComponentBeginOverlap(Sphere)
  (params (OverlappedComponent :type Primitive%20Component%20Object%20Reference) (OtherActor :type Actor%20Object%20Reference) (OtherComp :type Primitive%20Component%20Object%20Reference) (OtherBodyIndex :type Integer) (bFromSweep :type Boolean) (SweepResult :type Hit%20Result%20Structure%20%28by%20ref%29))
  ;[1 1 1] Apply gameplay effect
  (Class|ECMEffectActor|OnOverlap OtherActor))

(event EventBeginPlay)

(event Collision|EventActorBeginOverlap
  (params (OtherActor :type Actor%20Object%20Reference)))

(event EventTick
  (params (DeltaSeconds :type Float%20%28single-precision%29)))

(fn ConstructionScript
  ;[1 1 1] Construct from Data Asset
  (Utilities|FlowControl|Sequence
    (:then_0
      (Components|StaticMesh|SetStaticMesh)
      (Rendering|Material|SetMaterial))
    (:then_1
      (|SetGameplayEffect)
      (|ApplyGameplayEffectsPolicies))))